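; BP_FallingPlatform is a platform that starts falling two seconds after an actor overlap.
; The overlap event checks that player 0 is a BP_Character, not which actor overlapped, then sets a Fall flag after the delay.
; While Fall is set, Tick offsets the platform along Z by Direction times Speed, scaled by delta time, with no stop or reset.
; BeginPlay caches the player character, which is otherwise unused here.
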(event EventTick
  (params (DeltaSeconds :type Float%20%28single-precision%29))
  (if (Variables|Default|GetFall)
    (Transformation|AddActorWorldOffset (Math|Vector|MakeVector 0.0 0.0 (.z (* (* (Variables|Default|GetDirection) (Variables|Default|GetSpeed)) DeltaSeconds))))))

(event EventBeginPlay
  (bind _asbp_character (Utilities|Casting|CastToBP_Character (Game|GetPlayerCharacter 0)))
  (Variables|Default|SetCharacter _asbp_character))

(event Collision|EventActorBeginOverlap
  (params (OtherActor :type Actor%20Object%20Reference))
  (Utilities|Casting|CastToBP_Character (Game|GetPlayerCharacter 0))
  (Utilities|FlowControl|Delay 2.0)
  (Variables|Default|SetFall true))

(fn ConstructionScript)