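; A platform that damages the player after a charge-up on overlap, calling GameOver when Health reaches zero.
; A charge timeline tints the dynamic material and reverses when overlap ends, subtracting one Health only if it completes forward.
; A hit starts a timed cooldown with overlap events disabled and a recharge color timeline, then restarts charging if the player remains on it.
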(event EventBeginPlay
  (bind _asbp_character (Utilities|Casting|CastToBP_Character (Game|GetPlayerCharacter 0)))
  (Variables|Default|SetCharacter _asbp_character))

(event Collision|EventActorBeginOverlap
  (params (OtherActor :type Actor%20Object%20Reference))
  (if (not (Variables|Default|GetPlatfromOverlapRecharge)) :!label _label
    (bind _platformcolor (Timeline|PlatformCharge Play)
      (:Update
        (Rendering|Material|SetVectorParameterValue (Variables|Default|GetDynamicMaterial) "Color" _platformcolor :!class /Script/Engine.MaterialInstanceDynamic))
      (:Finished
        (if (not (< (Components|Timeline|GetPlaybackPosition (Variables|Default|GetPlatformCharge)) 1.0))
          (Utilities|FlowControl|Sequence
            (:then_0
              (bind _output_get (Variables|Default|SetColor "(R=1.000000,G=0.025053,B=0.118024,A=1.000000)"))
              (Rendering|Material|SetVectorParameterValue (Variables|Default|GetDynamicMaterial) "Color" _output_get :!class /Script/Engine.MaterialInstanceDynamic)
              (Utilities|FlowControl|Delay 0.2)
              (bind _platformcolor_2 (Timeline|PlatformRecharge Play)
                (:Update
                  (Rendering|Material|SetVectorParameterValue (Variables|Default|GetDynamicMaterial) "Color" _platformcolor_2 :!class /Script/Engine.MaterialInstanceDynamic))))
            (:then_1
              (Variables|/Game/Blueprints/BP_Character.BP_Character_C|SetHealth (Variables|Default|GetCharacter) (- (Variables|/Game/Blueprints/BP_Character.BP_Character_C|GetHealth (Variables|Default|GetCharacter)) 1))
              (if (== (Variables|/Game/Blueprints/BP_Character.BP_Character_C|GetHealth (Variables|Default|GetCharacter)) 0)
                (Default|GameOver (Variables|Default|GetCharacter))))
            (:then_2
              (Variables|Default|SetPlatfromOverlapRecharge true)
              (Variables|/Script/Engine.PrimitiveComponent|SetbGenerateOverlapEvents (Variables|Default|GetCollision%20Box) false)
              (Utilities|FlowControl|Delay 5.0)
              (Variables|/Script/Engine.PrimitiveComponent|SetbGenerateOverlapEvents (Variables|Default|GetCollision%20Box) true)
              (Variables|Default|SetPlatfromOverlapRecharge false)
              (Components|Timeline|SetPlaybackPosition (Variables|Default|GetPlatformCharge) 0.0 false true)
              (if (Collision|IsOverlappingActor (Variables|Default|GetCharacter) :!class /Script/Engine.Actor)
                (goto _label)))))))))

(event Collision|EventActorEndOverlap
  (params (OtherActor :type Actor%20Object%20Reference))
  (if (not (Variables|Default|GetPlatfromOverlapRecharge))
    (bind _platformcolor (Timeline|PlatformCharge Reverse)
      (:Update
        (Rendering|Material|SetVectorParameterValue (Variables|Default|GetDynamicMaterial) "Color" _platformcolor :!class /Script/Engine.MaterialInstanceDynamic))
      (:Finished
        (if (not (< (Components|Timeline|GetPlaybackPosition (Variables|Default|GetPlatformCharge)) 1.0))
          (Utilities|FlowControl|Sequence
            (:then_0
              (bind _output_get (Variables|Default|SetColor "(R=1.000000,G=0.025053,B=0.118024,A=1.000000)"))
              (Rendering|Material|SetVectorParameterValue (Variables|Default|GetDynamicMaterial) "Color" _output_get :!class /Script/Engine.MaterialInstanceDynamic)
              (Utilities|FlowControl|Delay 0.2)
              (bind _platformcolor_2 (Timeline|PlatformRecharge Play)
                (:Update
                  (Rendering|Material|SetVectorParameterValue (Variables|Default|GetDynamicMaterial) "Color" _platformcolor_2 :!class /Script/Engine.MaterialInstanceDynamic))))
            (:then_1
              (Variables|/Game/Blueprints/BP_Character.BP_Character_C|SetHealth (Variables|Default|GetCharacter) (- (Variables|/Game/Blueprints/BP_Character.BP_Character_C|GetHealth (Variables|Default|GetCharacter)) 1))
              (if (== (Variables|/Game/Blueprints/BP_Character.BP_Character_C|GetHealth (Variables|Default|GetCharacter)) 0)
                (Default|GameOver (Variables|Default|GetCharacter))))
            (:then_2
              (Variables|Default|SetPlatfromOverlapRecharge true)
              (Variables|/Script/Engine.PrimitiveComponent|SetbGenerateOverlapEvents (Variables|Default|GetCollision%20Box) false)
              (Utilities|FlowControl|Delay 5.0)
              (Variables|/Script/Engine.PrimitiveComponent|SetbGenerateOverlapEvents (Variables|Default|GetCollision%20Box) true)
              (Variables|Default|SetPlatfromOverlapRecharge false)
              (Components|Timeline|SetPlaybackPosition (Variables|Default|GetPlatformCharge) 0.0 false true)
              (if (Collision|IsOverlappingActor (Variables|Default|GetCharacter) :!class /Script/Engine.Actor)
                (if (not (Variables|Default|GetPlatfromOverlapRecharge))
                  (Timeline|PlatformCharge Play))))))))))

(fn ConstructionScript
  (bind _returnvalue (Rendering|Material|CreateDynamicMaterialInstance (Variables|Default|GetPlatform) 0 0 "None" :!class /Script/Engine.PrimitiveComponent))
  (bind _output_get (Variables|Default|SetDynamicMaterial _returnvalue))
  (Rendering|Material|SetVectorParameterValue _output_get "Color" (Variables|Default|GetColor) :!class /Script/Engine.MaterialInstanceDynamic))