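; BP_DamagePlatform_2 is a hazard platform that alternates between safe and damaging states on an endless timed loop.
; BeginPlay caches the player BP_Character, then toggles the Damage flag and recolors a dynamic material instance created in the construction script.
; DealDamage removes one Health when damage activates under an overlapping player or any overlap begins while active, calling GameOver at zero.
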(event EventBeginPlay
  (bind _asbp_character (Utilities|Casting|CastToBP_Character (Game|GetPlayerCharacter 0)))
  (Variables|Default|SetCharacter _asbp_character)
  (Variables|Default|SetDamage false :!label _label)
  (bind _output_get (Variables|Default|SetColor "(R=1.000000,G=0.223958,B=0.297961,A=1.000000)"))
  (Rendering|Material|SetVectorParameterValue (Variables|Default|GetDynamicMaterial) "Color" _output_get :!class /Script/Engine.MaterialInstanceDynamic)
  (Utilities|FlowControl|Delay 3.0)
  (Variables|Default|SetDamage true)
  (bind _output_get_2 (Variables|Default|SetColor "(R=1.000000,G=0.025053,B=0.118024,A=1.000000)"))
  (Rendering|Material|SetVectorParameterValue (Variables|Default|GetDynamicMaterial) "Color" _output_get_2 :!class /Script/Engine.MaterialInstanceDynamic)
  (if (Collision|IsOverlappingActor (Variables|Default|GetCharacter) :!class /Script/Engine.Actor)
    (CallFunction|DealDamage))
  (Utilities|FlowControl|Delay 2.0)
  (goto _label))

(event Collision|EventActorBeginOverlap
  (params (OtherActor :type Actor%20Object%20Reference))
  (if (Variables|Default|GetDamage)
    (CallFunction|DealDamage)))

(fn ConstructionScript
  (bind _returnvalue (Rendering|Material|CreateDynamicMaterialInstance (Variables|Default|GetPlatform) 0 0 "None" :!class /Script/Engine.PrimitiveComponent))
  (bind _output_get (Variables|Default|SetDynamicMaterial _returnvalue))
  (Rendering|Material|SetVectorParameterValue _output_get "Color" (Variables|Default|GetColor) :!class /Script/Engine.MaterialInstanceDynamic))

(fn DealDamage
  (Variables|/Game/Blueprints/BP_Character.BP_Character_C|SetHealth (Variables|Default|GetCharacter) (- (Variables|/Game/Blueprints/BP_Character.BP_Character_C|GetHealth (Variables|Default|GetCharacter)) 1))
  (if (== (Variables|/Game/Blueprints/BP_Character.BP_Character_C|GetHealth (Variables|Default|GetCharacter)) 0)
    (Default|GameOver (Variables|Default|GetCharacter))))