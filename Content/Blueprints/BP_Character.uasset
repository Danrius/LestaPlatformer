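; Player character Blueprint with camera-relative movement, look and jump input, plus a run stopwatch and end-of-game handling.
; StartStopwatch runs a looping one-second timer that updates minute and second counters and formats them into a Time string.
; Overlapping a KillZVolume destroys the actor and calls GameOver, which plays a death animation if the mesh is valid, pauses and shows the game-over widget.
; Victory pauses the stopwatch, disables movement and shows the victory widget.
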(event Custom|StartStopwatch
  (bind _returnvalue (Utilities|Time|SetTimerbyFunctionName 0 "Stopwatch" 1.0 true))
  (Variables|Default|SetStopwatchHandle _returnvalue))

(event Custom|GameOver
  (Input|SetInputModeUIOnly (Game|GetPlayerController 0) 0 "DoNotLock" false)
  (Variables|Character|GetMesh
    (:then
      (Pawn|Components|CharacterMovement|DisableMovement (Variables|Character|GetCharacterMovement))
      (Components|Animation|PlayAnimation (Variables|Character|GetMesh) "/Game/Assets/Character/Character_Anim_CharacterArmature_Death.Character_Anim_CharacterArmature_Death" false)
      (Utilities|FlowControl|Delay 0.8))
    (:else
      _))
  (Game|SetGamePaused true)
  (Viewport|RemoveAllWidgets)
  (bind _returnvalue (UserInterface|CreateWidget "/Game/Blueprints/WG_GameOver.WG_GameOver_C"))
  (UserInterface|Viewport|AddtoViewport _returnvalue 0)
  (Variables|/Script/Engine.PlayerController|SetbShowMouseCursor (Game|GetPlayerController 0) true))

(event Custom|Victory
  (Utilities|Time|PauseTimerbyHandle (Variables|Default|GetStopwatchHandle))
  (Pawn|Components|CharacterMovement|DisableMovement (Variables|Character|GetCharacterMovement))
  (Viewport|RemoveAllWidgets)
  (bind _returnvalue (UserInterface|CreateWidget "/Game/Blueprints/WG_Victory.WG_Victory_C"))
  (UserInterface|Viewport|AddtoViewport _returnvalue 0)
  (Input|SetInputModeUIOnly (Game|GetPlayerController 0) 0 "DoNotLock" false)
  (Variables|/Script/Engine.PlayerController|SetbShowMouseCursor (Game|GetPlayerController 0) true))

(event Collision|EventActorBeginOverlap
  (params (OtherActor :type Actor%20Object%20Reference))
  (Utilities|Casting|CastToKillZVolume OtherActor)
  (Actor|DestroyActor)
  (CallFunction|GameOver))

(event EventBeginPlay
  (Variables|Default|SetTime (Utilities|String|Append (Utilities|String|ToString(Text) (Utilities|Text|ToText(Integer) (Variables|Default|GetMinutes) false true 2 2)) ":" (Utilities|String|ToString(Text) (Utilities|Text|ToText(Integer) (Variables|Default|GetSeconds) false true 2 2)))))

(event Input|ActionEvents|InputActionJump
  (params (Key :type Key%20Structure :default "None"))
  (:Pressed
    (Character|Jump)))

(event Input|AxisEvents|InputAxisMoveForward&Backward
  (params (AxisValue :type Float%20%28single-precision%29))
  (bind _returnvalue (Pawn|GetControlRotation :!class /Script/Engine.Pawn))
  (bind _returnvalue_2 (Math|Rotator|MakeRotator 0.0 0.0 (.yaw _returnvalue)))
  (bind _returnvalue_3 (Math|Vector|GetForwardVector _returnvalue_2))
  (Pawn|Input|AddMovementInput (Math|Vector|MakeVector (.x _returnvalue_3) (.y _returnvalue_3) 0.0) AxisValue false))

(event Input|AxisEvents|InputAxisMoveLeft&Right
  (params (AxisValue :type Float%20%28single-precision%29))
  (bind _returnvalue (Pawn|GetControlRotation :!class /Script/Engine.Pawn))
  (bind _returnvalue_2 (Math|Rotator|MakeRotator 0.0 0.0 (.yaw _returnvalue)))
  (bind _returnvalue_3 (Math|Vector|GetRightVector _returnvalue_2))
  (Pawn|Input|AddMovementInput (Math|Vector|MakeVector (.x _returnvalue_3) (.y _returnvalue_3) 0.0) AxisValue false))

(event Input|AxisEvents|InputAxisCameraLeft&Right
  (params (AxisValue :type Float%20%28single-precision%29))
  (Pawn|Input|AddControllerYawInput AxisValue))

(event Input|AxisEvents|InputAxisCameraUp&Down
  (params (AxisValue :type Float%20%28single-precision%29))
  (Pawn|Input|AddControllerPitchInput AxisValue))

(fn ConstructionScript)

(fn Stopwatch
  (Math|Integer|IncrementInt (Variables|Default|GetSeconds)
    (:%20%20
      (if (== (Variables|Default|GetSeconds) 60)
        (Math|Integer|IncrementInt (Variables|Default|GetMinutes)
          (:%20%20
            (Variables|Default|SetSeconds 0))))
      (Variables|Default|SetTime (Utilities|String|Append (Utilities|String|ToString(Text) (Utilities|Text|ToText(Integer) (Variables|Default|GetMinutes) false true 2 2)) ":" (Utilities|String|ToString(Text) (Utilities|Text|ToText(Integer) (Variables|Default|GetSeconds) false true 2 2)))))))