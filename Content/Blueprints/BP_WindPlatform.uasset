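; Platform actor that pushes the player character with gusts of wind while something overlaps it.
; Overlap events toggle the wind without filtering the overlapping actor, and Tick moves the cached player character horizontally by direction and speed with a swept offset.
; While wind is active, a looping retriggerable delay picks one of four axis-aligned directions at random every two seconds.
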(event Custom|RandomWind
  (if (Variables|Default|GetWind) :!label _label
    (Utilities|FlowControl|RetriggerableDelay 2.0)
    (bind _output_get (Variables|Default|SetWindDirection (Utilities|Select :Index (Math|Random|RandomIntegerinRange 0 3) :Option%200 "NewEnumerator0" :Option%201 "NewEnumerator1" :Option%202 "NewEnumerator2" :Option%203 "NewEnumerator3")))
    (switch Utilities|FlowControl|Switch|SwitchonRandom_Wind _output_get
      (:NewEnumerator0
        (Variables|Default|SetDirection (Math|Vector|MakeVector 5e+01 0.0 0.0))
        (goto _label))
      (:NewEnumerator1
        (Variables|Default|SetDirection (Math|Vector|MakeVector -5e+01 0.0 0.0))
        (goto _label))
      (:NewEnumerator2
        (Variables|Default|SetDirection (Math|Vector|MakeVector 0.0 5e+01 0.0))
        (goto _label))
      (:NewEnumerator3
        (Variables|Default|SetDirection (Math|Vector|MakeVector 0.0 -5e+01 0.0))
        (goto _label)))))

(event EventTick
  (params (DeltaSeconds :type Float%20%28single-precision%29))
  (bind _speed (Variables|Default|GetSpeed))
  (bind _direction (Variables|Default|GetDirection))
  (bind _returnvalue (* _direction _speed))
  (bind _returnvalue_2 (* _returnvalue DeltaSeconds))
  (if (Variables|Default|GetWind)
    (Transformation|AddActorWorldOffset (Variables|Default|GetCharacter) (Math|Vector|MakeVector (.x _returnvalue_2) (.y _returnvalue_2) 0.0) true)))

(event EventBeginPlay
  (bind _asbp_character (Utilities|Casting|CastToBP_Character (Game|GetPlayerCharacter 0)))
  (Variables|Default|SetCharacter _asbp_character))

(event Collision|EventActorBeginOverlap
  (params (OtherActor :type Actor%20Object%20Reference))
  (Variables|Default|SetWind true)
  (CallFunction|RandomWind))

(event Collision|EventActorEndOverlap
  (params (OtherActor :type Actor%20Object%20Reference))
  (Variables|Default|SetWind false))

(fn ConstructionScript)